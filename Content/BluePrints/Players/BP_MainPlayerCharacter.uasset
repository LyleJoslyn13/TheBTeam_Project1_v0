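; BP_MainPlayerCharacter is a player character Blueprint that gains its dash ability from a component added at runtime.
; On BeginPlay it calls the parent, then adds and stores a BPC dash feature component with dashing enabled and itself as owner.
; Nodes adding face-the-mouse, rocket launcher and machine gun components are present but disconnected.
; Overlap and construction logic only forward to the parent class.
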(event `self.ReceiveBeginPlay`
  (`parent.ReceiveBeginPlay`)
  (bind _returnvalue (`AddComponent|NODE_AddBPC_DashFeature-1` :`owningCharacter` self))
  (set `self.BPC_DashFeature` _returnvalue))

(event `self.ReceiveActorBeginOverlap`
  (params (OtherActor :type "Actor Object Reference"))
  (`parent.ReceiveActorBeginOverlap` OtherActor))

(fn `UserConstructionScript`
  (`parent.UserConstructionScript`))