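; Police enemy character that chases the player's car and shoots at it.
; Each Tick, unless knocked back, it moves toward BP_Car's cube and, within attack range, spawns bullets aimed by yaw on a delay-based cooldown.
; Knockback takes damage from the car's machine gun component, then either reports the kill or launches the enemy, pausing pursuit via retriggerable delay.
; Generic damage can also destroy it, as does overlapping the car in monster truck mode.
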(event `self.ReceiveActorBeginOverlap`
  (params (OtherActor :type "Actor Object Reference"))
  (`parent.ReceiveActorBeginOverlap` null))

(event `self.ReceiveBeginPlay`
  (`parent.ReceiveBeginPlay`)
  (bind _aspawn (cast `Pawn` (`GameplayStatics.GetPlayerPawn` 0)))
  (set `self.BP_Car` _aspawn))

(event `self.ReceiveTick`
  (params (DeltaSeconds :type "Float (single-precision)"))
  (bind _returnvalue (`self.K2_GetActorLocation`))
  (`parent.ReceiveTick` DeltaSeconds)
  (if (not (`self.isKnockback`))
    (bind _returnvalue_2 (`GameplayStatics.GetActorOfClass` "/Game/Nathan/Player/BP_Car.BP_Car_C"))
    (`|AIMoveTo` self (`SceneComponent.K2_GetComponentLocation` (`/Game/Nathan/Player/BP_Car.Cube` _returnvalue_2)) null
      (:`then`
        (bind _returnvalue_3 (`GameplayStatics.GetActorOfClass` "/Game/Nathan/Player/BP_Car.BP_Car_C"))
        (if (and (`self.canFire`) (<= (`self.GetDistanceTo` (`self.BP_Car`)) (`self.AttackRange`)))
          (set `self.canFire` false)
          (bind (_returnvalue_roll _returnvalue_pitch _returnvalue_yaw) (`KismetMathLibrary.BreakRotator` (`KismetMathLibrary.FindLookAtRotation` _returnvalue (`self.K2_GetActorLocation` _returnvalue_3))))
          (`|SpawnActorFromClass` "/Game/BluePrints/Actors/BP_EnemyBullet.BP_EnemyBullet_C" (`KismetMathLibrary.MakeTransform` _returnvalue (`KismetMathLibrary.MakeRotator` 0.0 0.0 _returnvalue_yaw) (0.25 0.25 0.25)) "Undefined" "MultiplyWithRoot" null null)
          (`KismetSystemLibrary.Delay` 3.0)
          (set `self.canFire` true))))))

(event `self.ReceiveAnyDamage`
  (params (Damage :type "Float (single-precision)") (DamageType :type "DamageType Object Reference") (InstigatedBy :type "Controller Object Reference") (DamageCauser :type "Actor Object Reference"))
  (set `self.CurrentHealth` (- (`self.CurrentHealth`) Damage))
  (if (<= (`self.CurrentHealth`) 0.0)
    (`self.K2_DestroyActor`)))

(event `self.Knockback`
  (params (Impulse :type "Vector Structure"))
  (bind _returnvalue (`self.GetComponentByClass` (`self.BP_Car`) "/Game/BluePrints/ActorComponents/BPC_MachineGun.BPC_MachineGun_C"))
  (`MovementComponent.StopMovementImmediately` (`self.CharacterMovement`))
  (bind _updatedhealth (`/Game/BluePrints/ActorComponents/BPC_MachineGun.DealDamage` _returnvalue (`self.CurrentHealth`)))
  (bind _output_get (set `self.CurrentHealth` _updatedhealth))
  (if (<= _output_get 0.0)
    (set `self.isDead` true)
    (`/Game/BluePrints/ActorComponents/BPC_MachineGun.EnemyKilled` _returnvalue)
    (`self.K2_DestroyActor`)
    (else
      (`self.LaunchCharacter` Impulse true)
      (set `self.isKnockback` true)
      (`KismetSystemLibrary.RetriggerableDelay` 0.35)
      (set `self.isKnockback` false))))

(event `self.Box.OnComponentBeginOverlap`
  (params (OverlappedComponent :type "PrimitiveComponent Object Reference") (OtherActor :type "Actor Object Reference") (OtherComp :type "PrimitiveComponent Object Reference") (OtherBodyIndex :type Integer) (bFromSweep :type Boolean) (SweepResult :type "HitResult Structure (by ref)"))
  (bind _bp_car (`self.BP_Car`))
  (if (== OtherActor _bp_car)
    (if (`/Game/BluePrints/ActorComponents/BPC_MonsterTruck.isMonsterTruck` (`self.GetComponentByClass` _bp_car "/Game/BluePrints/ActorComponents/BPC_MonsterTruck.BPC_MonsterTruck_C"))
      (`KismetSystemLibrary.PrintString` "KNOCKBACK")
      (`self.K2_DestroyActor`))))

(fn `GetIsDead`
  (returns (isDead :type Boolean))
  (return (`self.isDead`)))

(fn `UserConstructionScript`
  (`parent.UserConstructionScript`))