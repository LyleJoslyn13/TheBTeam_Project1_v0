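; Common enemy character that chases the player with AI MoveTo, reissued every Tick unless it is being knocked back.
; Its Knockback event stops movement and updates health through DealDamage on the player's BPC_MachineGun component.
; At zero health it flags itself dead, calls EnemyKilled on that component (noted as not working) and destroys itself.
; Otherwise it launches by the impulse and pauses chasing through a short retriggerable delay.
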(event `self.ReceiveTick`
  (params (DeltaSeconds :type "Float (single-precision)"))
  (`parent.ReceiveTick` DeltaSeconds)
  (if (not (`self.isKnockback`))
    (`|AIMoveTo` self (0.0 0.0 0.0) (`GameplayStatics.GetPlayerCharacter` 0)
      (:`OnSuccess`
        (`KismetSystemLibrary.PrintString` "yay")))))

(event `/Game/BluePrints/Interfaces/BPI_EnemyInteractions.Knockback`
  (params (Impulse :type "Vector Structure"))
  (bind _returnvalue (`self.GetComponentByClass` (`GameplayStatics.GetPlayerCharacter` 0) "/Game/BluePrints/ActorComponents/BPC_MachineGun.BPC_MachineGun_C"))
  (`MovementComponent.StopMovementImmediately` (`self.CharacterMovement`))
  (bind _updatedhealth (`/Game/BluePrints/ActorComponents/BPC_MachineGun.DealDamage` _returnvalue (`self.CurrentHealth`)))
  (bind _output_get (set `self.CurrentHealth` _updatedhealth))
  (if (<= _output_get 0.0)
    (set `self.isDead` true)
    (`/Game/BluePrints/ActorComponents/BPC_MachineGun.EnemyKilled` _returnvalue) ; THIS DOESNT WORK
    (`self.K2_DestroyActor`)
    (else
      (`self.LaunchCharacter` Impulse true)
      (set `self.isKnockback` true)
      (`KismetSystemLibrary.RetriggerableDelay` 0.35)
      (set `self.isKnockback` false))))

(fn `GetIsDead`
  (returns (isDead :type Boolean))
  (return (`self.isDead`)))

(fn `UserConstructionScript`
  (`parent.UserConstructionScript`))