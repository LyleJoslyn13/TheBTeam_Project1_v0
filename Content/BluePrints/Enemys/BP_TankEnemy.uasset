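; Enemy tank pawn that chases the player's BP_Car, shoots at it and damages it on contact.
; When PawnSensing sees the car, the tank yaws its body and actor toward it and uses AI MoveTo to approach within an acceptance radius.
; The same sight event spawns BP_Bullet at BulletSpawn after a Delay, which paces the firing.
; Overlapping the player lowers the car's CurrentHealth, with a CanDamage flag and delay as cooldown.
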(event `self.PawnSensing.OnSeePawn`
  (params (Pawn :type "Pawn Object Reference"))
  (bind _asbp_car (cast `/Game/Nathan/Player/BP_Car` Pawn))
  (`|ExecutionSequence`
    (:`then_0`
      (bind (_returnvalue_roll _returnvalue_pitch _returnvalue_yaw) (`KismetMathLibrary.BreakRotator` (`KismetMathLibrary.RInterpTo` (`self.K2_GetActorRotation`) (`KismetMathLibrary.FindLookAtRotation` (`self.K2_GetActorLocation`) (`self.K2_GetActorLocation` _asbp_car)) (`GameplayStatics.GetWorldDeltaSeconds`) 100.0)))
      (`SceneComponent.K2_SetWorldRotation` (`self.body`) (`KismetMathLibrary.MakeRotator` 0.0 0.0 _returnvalue_yaw) false false)
      (`self.K2_SetActorRotation` (`KismetMathLibrary.MakeRotator` 0.0 0.0 _returnvalue_yaw))
      (bind (_returnvalue_x _returnvalue_y) (`KismetMathLibrary.BreakVector` (`self.K2_GetActorLocation` _asbp_car)))
      (`|AIMoveTo` self (`KismetMathLibrary.MakeVector` _returnvalue_x _returnvalue_y) null 800.0))
    (:`then_1`
      (`KismetSystemLibrary.Delay` 3.0)
      (`|SpawnActorFromClass` "/Game/BluePrints/Actors/BP_Bullet.BP_Bullet_C" (`SceneComponent.K2_GetComponentToWorld` (`self.bulletSpawn`)) "AlwaysSpawn" "MultiplyWithRoot" null null))))

(event `self.ReceiveActorBeginOverlap`
  (params (OtherActor :type "Actor Object Reference"))
  (bind _returnvalue (`GameplayStatics.GetPlayerPawn` 0))
  (if (== OtherActor _returnvalue)
    (if (`self.CanDamage`)
      (bind _asbp_car (cast `/Game/Nathan/Player/BP_Car` _returnvalue))
      (set `/Game/Nathan/Player/BP_Car.CurrentHealth` (- (`/Game/Nathan/Player/BP_Car.CurrentHealth` _asbp_car) 10.0) _asbp_car)
      (set `self.CanDamage` false)
      (`KismetSystemLibrary.Delay` 3.0)
      (set `self.CanDamage` true))))

(fn `UserConstructionScript`
  (`parent.UserConstructionScript`))