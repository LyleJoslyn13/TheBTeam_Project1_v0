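; Destructible oil tanker actor that takes damage from bullets and player ramming, catches fire at low health and explodes.
; Box collision events reduce health, with ram handling gated by a timed IsRammed flag, then reveal fire and start the explosion at zero.
; Next-tick delay loops drive timers and grow the explosion sphere before destruction, while it repeatedly drains overlapping player car health.
; CheckHealth holds an uncalled, delay-free variant of the explosion logic.
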(event `self.ReceiveBeginPlay`
  (bind _asbp_car (cast `/Game/Nathan/Player/BP_Car` (`GameplayStatics.GetPlayerPawn` 0)))
  (set `self.As BP Car` _asbp_car))

(event `self.Box.OnComponentBeginOverlap`
  (params (OverlappedComponent :type "PrimitiveComponent Object Reference") (OtherActor :type "Actor Object Reference") (OtherComp :type "PrimitiveComponent Object Reference") (OtherBodyIndex :type Integer) (bFromSweep :type Boolean) (SweepResult :type "HitResult Structure (by ref)"))
  (bind _explosiontime (`self.ExplosionTime`))
  (bind _sphere (`self.Sphere`))
  (bind (_returnvalue_location _returnvalue_rotation) (`KismetMathLibrary.BreakTransform` (`SceneComponent.GetRelativeTransform` _sphere)))
  (bind _returnvalue (`KismetMathLibrary.MapRangeClamped` _explosiontime 0.0 2.0 2.0 10.0))
  (if (`self.isExploading`)
    _
    (elif (`self.isRammed`)
      (if (== OtherActor (`GameplayStatics.GetPlayerPawn` 0))
        (`KismetSystemLibrary.PrintString` "RAMMED")
        (set `self.CurrentHealth` (- (`self.CurrentHealth`) (`self.CarDamage`)))
        (`|ExecutionSequence`
          (:`then_0`
            (set `self.isRammed` true)
            (bind _output_get (set `self.RammedTime` (+ (`self.RammedTime`) (`GameplayStatics.GetWorldDeltaSeconds`)) :!label _label))
            (if (>= _output_get (`self.MaxRammedTime`))
              (set `self.isRammed` false)
              (else
                (`KismetSystemLibrary.DelayUntilNextTick`)
                (goto _label))))
          (:`then_1`
            (if (not (>= (`self.CurrentHealth`) (`self.SmokeMin`))) :!label _label_2
              (`KismetSystemLibrary.PrintString` "fire")
              (`SceneComponent.SetVisibility` (`self.Fire`) true false)
              (`SceneComponent.SetVisibility` (`self.Fire1`) true false)
              (if (<= (`self.CurrentHealth`) 0.0)
                (`KismetSystemLibrary.PrintString` "isDead")
                (`SceneComponent.SetVisibility` _sphere true false)
                (bind _output_get_2 (set `self.isExploading` true))
                (if _output_get_2 :!label _label_3
                  (`SceneComponent.K2_SetRelativeTransform` _sphere (`KismetMathLibrary.MakeTransform` _returnvalue_location _returnvalue_rotation (`KismetMathLibrary.MakeVector` _returnvalue _returnvalue _returnvalue)) false false)
                  (bind _output_get_3 (set `self.ExplosionTime` (+ (`GameplayStatics.GetWorldDeltaSeconds`) _explosiontime)))
                  (if (>= _output_get_3 (`self.MaxExplosionTime`))
                    (set `self.isExploading` false)
                    (`self.K2_DestroyActor`)
                    (else
                      (`KismetSystemLibrary.DelayUntilNextTick`)
                      (goto _label_3))))))))))))

(event `self.Box.OnComponentHit`
  (params (HitComponent :type "PrimitiveComponent Object Reference") (OtherActor :type "Actor Object Reference") (OtherComp :type "PrimitiveComponent Object Reference") (NormalImpulse :type "Vector Structure") (Hit :type "HitResult Structure (by ref)"))
  (if (`self.isExploading`)
    _
    (elif (== (`GameplayStatics.GetObjectClass` OtherActor) (`self.Bullet`))
      (set `self.CurrentHealth` (- (`self.CurrentHealth`) (`self.BulletDamage`)))
      (goto _label_2))))

(event `self.Sphere.OnComponentBeginOverlap`
  (params (OverlappedComponent :type "PrimitiveComponent Object Reference") (OtherActor :type "Actor Object Reference") (OtherComp :type "PrimitiveComponent Object Reference") (OtherBodyIndex :type Integer) (bFromSweep :type Boolean) (SweepResult :type "HitResult Structure (by ref)"))
  (bind _returnvalue (`GameplayStatics.GetPlayerPawn` 0))
  (bind _as_bp_car (`self.As BP Car`))
  (bind _currenthealth (`/Game/Nathan/Player/BP_Car.CurrentHealth` _as_bp_car))
  (if (== OtherActor _returnvalue)
    (if (`self.isExploading`)
      (if (`PrimitiveComponent.IsOverlappingActor` (`self.Sphere`) _returnvalue) :!label _label_4
        (`KismetSystemLibrary.PrintString` (`KismetStringLibrary.Conv_DoubleToString` _currenthealth))
        (bind _result (`/Engine/EditorBlueprintResources/StandardMacros.DecrementFloat` _currenthealth)
          (:`  `
            (set `/Game/Nathan/Player/BP_Car.CurrentHealth` _result _as_bp_car)
            (`KismetSystemLibrary.Delay` 0.1)
            (goto _label_4)))))))

(fn `CheckHealth`
  (bind _explosiontime (`self.ExplosionTime`))
  (bind _sphere (`self.Sphere`))
  (bind _returnvalue (`KismetMathLibrary.MapRangeClamped` _explosiontime 0.0 2.0 2.0 4.0))
  (if (not (>= (`self.CurrentHealth`) (`self.SmokeMin`)))
    (`KismetSystemLibrary.PrintString` "fire")
    (`SceneComponent.SetVisibility` (`self.Fire`) true false)
    (`SceneComponent.SetVisibility` (`self.Fire1`) true false)
    (if (<= (`self.CurrentHealth`) 0.0)
      (`KismetSystemLibrary.PrintString` "isDead")
      (`SceneComponent.SetVisibility` _sphere true false)
      (bind _output_get (set `self.isExploading` true))
      (if _output_get :!label _label
        (`SceneComponent.SetRelativeScale3D` _sphere (`KismetMathLibrary.MakeVector` _returnvalue _returnvalue _returnvalue))
        (if (>= (+ _explosiontime (`GameplayStatics.GetWorldDeltaSeconds`)) (`self.MaxExplosionTime`))
          (set `self.isExploading` false)
          (`self.K2_DestroyActor`)
          (else
            (goto _label)))))))

(fn `UserConstructionScript`)