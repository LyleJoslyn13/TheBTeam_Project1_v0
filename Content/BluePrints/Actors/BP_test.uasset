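; Test actor that sketches timed bridge open/close logic, with no movement implemented.
; OpenBridge accumulates delta time through a next-tick delay loop instead of Event Tick, sets IsOpen after five seconds, then calls CloseBridge following a retriggerable delay.
; CloseBridge only prints a debug string when open, otherwise calls OpenBridge.
; The toggle branch is unreachable, the MapRangeClamped node is unused, and BeginPlay and overlap events are disabled.
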(event `OpenBridge`
  (if (`self.isOpen`) :!label _label
    (`KismetSystemLibrary.RetriggerableDelay` 5.0)
    (`self.CloseBridge`)
    (else
      (bind _output_get (set `self.AnimationTIme` (+ (`self.AnimationTIme`) (`GameplayStatics.GetWorldDeltaSeconds`))))
      (if (>= _output_get 5.0)
        (set `self.isOpen` true)
        (set `self.AnimationTIme` 0.0))
      (`KismetSystemLibrary.DelayUntilNextTick`)
      (goto _label))))

(event `CloseBridge`
  (if (`self.isOpen`)
    (`KismetSystemLibrary.PrintString` "Hello")
    (else
      (`self.OpenBridge`))))

(fn `UserConstructionScript`)