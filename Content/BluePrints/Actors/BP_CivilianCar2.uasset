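; BP_CivilianCar2 is an AI civilian car that drives toward a navmesh point projected ahead of its spawn.
; The BreakCheck overlap stops it for civilians and stoplights, and destroys it on leaving a BP_Boundary.
; First non-lethal damage retargets it once to a random BP_EscapePoint and flags it fleeing, so it keeps moving while blocked.
; Tick reissues movement each frame, and depleted health destroys the car.
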(event `self.ReceiveBeginPlay`
  (set `self.movementTarget` (`NavigationSystemV1.K2_ProjectPointToNavigation` (+ (* (`self.GetActorForwardVector`) 8000.0) (`self.K2_GetActorLocation`)) null null (`KismetMathLibrary.Conv_DoubleToVector` 2000.0))))

(event `self.BreakCheck.OnComponentBeginOverlap`
  (params (OverlappedComponent :type "PrimitiveComponent Object Reference") (OtherActor :type "Actor Object Reference") (OtherComp :type "PrimitiveComponent Object Reference") (OtherBodyIndex :type Integer) (bFromSweep :type Boolean) (SweepResult :type "HitResult Structure (by ref)"))
  (`|ExecutionSequence`
    (:`then_0`
      (cast `/Game/BluePrints/Actors/BP_Civilian` OtherActor))
    (:`then_1`
      (cast `/Game/BluePrints/Actors/BP_Stoplight` OtherActor)))
  (set `self.canDrive` false))

(event `self.BreakCheck.OnComponentEndOverlap`
  (params (OverlappedComponent :type "PrimitiveComponent Object Reference") (OtherActor :type "Actor Object Reference") (OtherComp :type "PrimitiveComponent Object Reference") (OtherBodyIndex :type Integer))
  (`|ExecutionSequence`
    (:`then_0`
      (cast `/Game/BluePrints/Actors/BP_Civilian` OtherActor)
      (set `self.canDrive` true :!label _label))
    (:`then_1`
      (cast `/Game/BluePrints/Actors/BP_Stoplight` OtherActor)
      (goto _label))
    (:`then_2`
      (cast `/Game/BluePrints/Actors/BP_Boundary` OtherActor)
      (`self.K2_DestroyActor`))))

(event `self.ReceiveTick`
  (params (DeltaSeconds :type "Float (single-precision)"))
  (`|ExecutionSequence`
    (:`then_0`
      (if (`self.canDrive`)
        (`AIBlueprintHelperLibrary.SimpleMoveToLocation` (`self.GetController`) (`self.movementTarget`))
        (elif (`self.isFleeing`)
          (`|AIMoveTo` self (`self.movementTarget`) null)
          (else
            (`MovementComponent.StopMovementImmediately` (`self.CharacterMovement`))))))))

(event `self.ReceiveAnyDamage`
  (params (Damage :type "Float (single-precision)") (DamageType :type "DamageType Object Reference") (InstigatedBy :type "Controller Object Reference") (DamageCauser :type "Actor Object Reference"))
  (set `self.CurrentHealth` (- (`self.CurrentHealth`) Damage))
  (if (<= (`self.CurrentHealth`) 0.0)
    (`self.K2_DestroyActor`)
    (else
      (`/Engine/EditorBlueprintResources/StandardMacros.DoOnce` false
        (:`Completed`
          (bind _outactors (`GameplayStatics.GetAllActorsOfClass` "/Game/BluePrints/Actors/BP_EscapePoint.BP_EscapePoint_C"))
          (set `self.movementTarget` (`NavigationSystemV1.K2_ProjectPointToNavigation` (`self.K2_GetActorLocation` (`KismetArrayLibrary.Array_Random` _outactors)) null null (`KismetMathLibrary.Conv_DoubleToVector` 300.0)))
          (set `self.isFleeing` true))))))

(fn `UserConstructionScript`)