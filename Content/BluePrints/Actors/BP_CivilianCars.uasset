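; Civilian car that drives straight ahead, brakes for civilians and stoplights, and can be destroyed by damage.
; BeginPlay sets a target far along its forward vector, and Tick reissues SimpleMoveToLocation toward it while CanDrive is true.
; BreakCheck overlaps clear CanDrive and end overlaps restore it, while ending overlap with a boundary destroys the car.
; Physics impulse nodes on CarBase are left unconnected.
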(event `self.ReceiveBeginPlay`
  (set `self.movementTarget` (+ (* (`self.GetActorForwardVector`) 8000.0) (`self.K2_GetActorLocation`))))

(event `self.ReceiveTick`
  (params (DeltaSeconds :type "Float (single-precision)"))
  (if (`self.canDrive`)
    (`AIBlueprintHelperLibrary.SimpleMoveToLocation` (`self.GetController`) (`self.movementTarget`))))

(event `self.ReceiveAnyDamage`
  (params (Damage :type "Float (single-precision)") (DamageType :type "DamageType Object Reference") (InstigatedBy :type "Controller Object Reference") (DamageCauser :type "Actor Object Reference"))
  (set `self.CurrentHealth` (- (`self.CurrentHealth`) Damage))
  (if (<= (`self.CurrentHealth`) 0.0)
    (`self.K2_DestroyActor`)))

(event `self.BreakCheck.OnComponentBeginOverlap`
  (params (OverlappedComponent :type "PrimitiveComponent Object Reference") (OtherActor :type "Actor Object Reference") (OtherComp :type "PrimitiveComponent Object Reference") (OtherBodyIndex :type Integer) (bFromSweep :type Boolean) (SweepResult :type "HitResult Structure (by ref)"))
  (`|ExecutionSequence`
    (:`then_0`
      (cast `/Game/BluePrints/Actors/BP_Civilian` OtherActor))
    (:`then_1`
      (cast `/Game/BluePrints/Actors/BP_Stoplight` OtherActor)))
  (set `self.canDrive` false))

(event `self.BreakCheck.OnComponentEndOverlap`
  (params (OverlappedComponent :type "PrimitiveComponent Object Reference") (OtherActor :type "Actor Object Reference") (OtherComp :type "PrimitiveComponent Object Reference") (OtherBodyIndex :type Integer))
  (`|ExecutionSequence`
    (:`then_0`
      (cast `/Game/BluePrints/Actors/BP_Civilian` OtherActor)
      (set `self.canDrive` true :!label _label))
    (:`then_1`
      (cast `/Game/BluePrints/Actors/BP_Stoplight` OtherActor)
      (goto _label))
    (:`then_2`
      (cast `/Game/BluePrints/Actors/BP_Boundary` OtherActor)
      (`self.K2_DestroyActor`))))

(fn `UserConstructionScript`)