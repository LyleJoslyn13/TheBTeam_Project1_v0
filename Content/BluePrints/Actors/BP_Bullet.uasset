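; BP_Bullet is a projectile actor that explodes on overlap or after a three-second fuse.
; Both triggers run the same duplicated sequence: expand the collision Sphere to a large blast radius, zero the ProjectileMovement velocity and activate the NSExplosion effect.
; The actor destroys itself after a short delay, and no damage is applied in this graph.
; The overlap path has no guard, so the enlarged sphere can retrigger it.
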(event `self.ReceiveBeginPlay`
  (`KismetSystemLibrary.Delay` 3.0)
  (`SphereComponent.SetSphereRadius` (`self.Sphere`) 1000.0 true)
  (`ProjectileMovementComponent.SetVelocityInLocalSpace` (`self.ProjectileMovement`) (0.0 0.0 0.0))
  (`ActorComponent.Activate` (`self.NS_explosion`) false)
  (`KismetSystemLibrary.Delay` 0.5)
  (`self.K2_DestroyActor`))

(event `self.Sphere.OnComponentBeginOverlap`
  (params (OverlappedComponent :type "PrimitiveComponent Object Reference") (OtherActor :type "Actor Object Reference") (OtherComp :type "PrimitiveComponent Object Reference") (OtherBodyIndex :type Integer) (bFromSweep :type Boolean) (SweepResult :type "HitResult Structure (by ref)"))
  (`SphereComponent.SetSphereRadius` (`self.Sphere`) 1000.0 true)
  (`ProjectileMovementComponent.SetVelocityInLocalSpace` (`self.ProjectileMovement`) (0.0 0.0 0.0))
  (`ActorComponent.Activate` (`self.NS_explosion`) false)
  (`KismetSystemLibrary.Delay` 0.5)
  (`self.K2_DestroyActor`))

(fn `UserConstructionScript`)