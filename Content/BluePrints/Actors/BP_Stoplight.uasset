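; BP_Stoplight is a timed stoplight actor that alternates two pairs of box components between raised and lowered positions.
; From BeginPlay, it waits on a fixed delay, then shifts Box2 and Box3 up while Box and Box1 move down, and reverses this after another delay.
; A custom Repeater event loops back to the first delay, cycling endlessly with instant world-space Z offsets rather than interpolation.
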(event `self.ReceiveBeginPlay`
  (bind (_returnvalue_x _returnvalue_y _returnvalue_z) (`KismetMathLibrary.BreakVector` (`SceneComponent.K2_GetComponentLocation` (`self.Box2`))))
  (bind (_returnvalue_x_2 _returnvalue_y_2 _returnvalue_z_2) (`KismetMathLibrary.BreakVector` (`SceneComponent.K2_GetComponentLocation` (`self.Box3`))))
  (bind (_returnvalue_x_3 _returnvalue_y_3 _returnvalue_z_3) (`KismetMathLibrary.BreakVector` (`SceneComponent.K2_GetComponentLocation` (`self.Box2`))))
  (bind (_returnvalue_x_4 _returnvalue_y_4 _returnvalue_z_4) (`KismetMathLibrary.BreakVector` (`SceneComponent.K2_GetComponentLocation` (`self.Box3`))))
  (bind (_returnvalue_x_5 _returnvalue_y_5 _returnvalue_z_5) (`KismetMathLibrary.BreakVector` (`SceneComponent.K2_GetComponentLocation` (`self.Box`))))
  (bind (_returnvalue_x_6 _returnvalue_y_6 _returnvalue_z_6) (`KismetMathLibrary.BreakVector` (`SceneComponent.K2_GetComponentLocation` (`self.Box1`))))
  (bind (_returnvalue_x_7 _returnvalue_y_7 _returnvalue_z_7) (`KismetMathLibrary.BreakVector` (`SceneComponent.K2_GetComponentLocation` (`self.Box1`))))
  (bind (_returnvalue_x_8 _returnvalue_y_8 _returnvalue_z_8) (`KismetMathLibrary.BreakVector` (`SceneComponent.K2_GetComponentLocation` (`self.Box`))))
  (`KismetSystemLibrary.Delay` 5.0 :!label _label)
  (`SceneComponent.K2_SetWorldLocation` (`self.Box2`) (`KismetMathLibrary.MakeVector` _returnvalue_x_3 _returnvalue_y_3 (+ _returnvalue_z_3 400.0)) false false)
  (`SceneComponent.K2_SetWorldLocation` (`self.Box3`) (`KismetMathLibrary.MakeVector` _returnvalue_x_4 _returnvalue_y_4 (+ _returnvalue_z_4 400.0)) false false)
  (`SceneComponent.K2_SetWorldLocation` (`self.Box`) (`KismetMathLibrary.MakeVector` _returnvalue_x_5 _returnvalue_y_5 (- _returnvalue_z_5 400.0)) false false)
  (`SceneComponent.K2_SetWorldLocation` (`self.Box1`) (`KismetMathLibrary.MakeVector` _returnvalue_x_6 _returnvalue_y_6 (- _returnvalue_z_6 400.0)) false false)
  (`KismetSystemLibrary.Delay` 5.0)
  (`SceneComponent.K2_SetWorldLocation` (`self.Box2`) (`KismetMathLibrary.MakeVector` _returnvalue_x _returnvalue_y (- _returnvalue_z 400.0)) false false)
  (`SceneComponent.K2_SetWorldLocation` (`self.Box3`) (`KismetMathLibrary.MakeVector` _returnvalue_x_2 _returnvalue_y_2 (- _returnvalue_z_2 400.0)) false false)
  (`SceneComponent.K2_SetWorldLocation` (`self.Box`) (`KismetMathLibrary.MakeVector` _returnvalue_x_8 _returnvalue_y_8 (+ _returnvalue_z_8 400.0)) false false)
  (`SceneComponent.K2_SetWorldLocation` (`self.Box1`) (`KismetMathLibrary.MakeVector` _returnvalue_x_7 _returnvalue_y_7 (+ _returnvalue_z_7 400.0)) false false)
  (`self.Repeater`))

(event `Repeater`
  (goto _label))

(fn `UserConstructionScript`)