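; BP_Civilian is a self-driving traffic actor that moves forward and halts for stoplights and other civilians.
; Each Tick it gradually accelerates or brakes more sharply based on CanDrive, then applies a swept forward offset to its root, without frame-time scaling.
; CollisionBox overlaps with BP_Civilian or BP_Stoplight clear CanDrive, and ending either overlap sets it again.
; Ending overlap with a BP_Boundary destroys the actor.
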(event `self.ReceiveTick`
  (params (DeltaSeconds :type "Float (single-precision)"))
  (bind _defaultsceneroot (`self.DefaultSceneRoot`))
  (if (`self.canDrive`)
    (set `self.speed` (`KismetMathLibrary.FClamp` (+ (`self.speed`) 0.005) 0.0 7.0))
    (else
      (set `self.speed` (`KismetMathLibrary.FClamp` (- (`self.speed`) 0.1) 0.0 7.0))))
  (`SceneComponent.K2_AddWorldOffset` _defaultsceneroot (* (`SceneComponent.GetForwardVector` _defaultsceneroot) (`self.speed`)) true false))

(event `self.CollisionBox.OnComponentBeginOverlap`
  (params (OverlappedComponent :type "PrimitiveComponent Object Reference") (OtherActor :type "Actor Object Reference") (OtherComp :type "PrimitiveComponent Object Reference") (OtherBodyIndex :type Integer) (bFromSweep :type Boolean) (SweepResult :type "HitResult Structure (by ref)"))
  (`|ExecutionSequence`
    (:`then_0`
      (cast `/Game/BluePrints/Actors/BP_Civilian` OtherActor))
    (:`then_1`
      (cast `/Game/BluePrints/Actors/BP_Stoplight` OtherActor)))
  (set `self.canDrive` false))

(event `self.CollisionBox.OnComponentEndOverlap`
  (params (OverlappedComponent :type "PrimitiveComponent Object Reference") (OtherActor :type "Actor Object Reference") (OtherComp :type "PrimitiveComponent Object Reference") (OtherBodyIndex :type Integer))
  (`|ExecutionSequence`
    (:`then_0`
      (cast `/Game/BluePrints/Actors/BP_Civilian` OtherActor)
      (set `self.canDrive` true :!label _label))
    (:`then_1`
      (cast `/Game/BluePrints/Actors/BP_Stoplight` OtherActor)
      (goto _label))
    (:`then_2`
      (cast `/Game/BluePrints/Actors/BP_Boundary` OtherActor)
      (`self.K2_DestroyActor`))))

(fn `UserConstructionScript`)