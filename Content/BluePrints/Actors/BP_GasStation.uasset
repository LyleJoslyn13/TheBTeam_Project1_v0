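; BP_GasStation is a gas station actor that repaints a passing BP_Car with a random material, then goes on cooldown.
; When a car enters the trigger Box while GasReady is true, its Cube gets a material from RandColor and the Roof switches to the gas-down material.
; When a car leaves, GasReady clears and a 30-second Delay runs before restoring it and the ready Roof material.
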(event `self.Box.OnComponentBeginOverlap`
  (params (OverlappedComponent :type "PrimitiveComponent Object Reference") (OtherActor :type "Actor Object Reference") (OtherComp :type "PrimitiveComponent Object Reference") (OtherBodyIndex :type Integer) (bFromSweep :type Boolean) (SweepResult :type "HitResult Structure (by ref)"))
  (if (`self.gasReady`)
    (bind _asbp_car (cast `/Game/Nathan/Player/BP_Car` OtherActor))
    (`PrimitiveComponent.SetMaterial` (`/Game/Nathan/Player/BP_Car.Cube` _asbp_car) 0 (`KismetArrayLibrary.Array_Random` (`self.randColor`)))
    (`PrimitiveComponent.SetMaterial` (`self.Roof`) 0 "/Game/Art/Materials/M_GasDown.M_GasDown")))

(event `self.Box.OnComponentEndOverlap`
  (params (OverlappedComponent :type "PrimitiveComponent Object Reference") (OtherActor :type "Actor Object Reference") (OtherComp :type "PrimitiveComponent Object Reference") (OtherBodyIndex :type Integer))
  (cast `/Game/Nathan/Player/BP_Car` OtherActor)
  (set `self.gasReady` false)
  (`KismetSystemLibrary.Delay` 30.0)
  (set `self.gasReady` true)
  (`PrimitiveComponent.SetMaterial` (`self.Roof`) 0 "/Game/Art/Materials/M_GasReady.M_GasReady"))

(fn `UserConstructionScript`)