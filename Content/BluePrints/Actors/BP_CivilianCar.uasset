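; BP_CivilianCar is a civilian traffic car that drives forward and halts for civilians and stoplights.
; While CanDrive is set, Tick zeroes the capsule's velocity, then applies an impulse built from forward vector plus world location.
; Box overlaps with BP_Civilian or BP_Stoplight toggle CanDrive, and ending overlap with BP_Boundary destroys the car.
; Speed ramping and AI MoveTo logic are disconnected, leaving BeginPlay's MovementTarget without effect.
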(event `self.ReceiveTick`
  (params (DeltaSeconds :type "Float (single-precision)"))
  (bind _capsulecomponent (`self.CapsuleComponent`))
  (if (`self.canDrive`)
    (`PrimitiveComponent.SetPhysicsLinearVelocity` _capsulecomponent (0.0 0.0 0.0) false "None")
    (`PrimitiveComponent.AddImpulse` _capsulecomponent (+ (* (`self.GetActorForwardVector`) 100000.0) (`self.K2_GetActorLocation`)) "None" false)))

(event `self.ReceiveBeginPlay`
  (set `self.movementTarget` (+ (* (`self.GetActorForwardVector`) 8000.0) (`self.K2_GetActorLocation`))))

(event `self.Box.OnComponentBeginOverlap`
  (params (OverlappedComponent :type "PrimitiveComponent Object Reference") (OtherActor :type "Actor Object Reference") (OtherComp :type "PrimitiveComponent Object Reference") (OtherBodyIndex :type Integer) (bFromSweep :type Boolean) (SweepResult :type "HitResult Structure (by ref)"))
  (`|ExecutionSequence`
    (:`then_0`
      (cast `/Game/BluePrints/Actors/BP_Civilian` OtherActor))
    (:`then_1`
      (cast `/Game/BluePrints/Actors/BP_Stoplight` OtherActor)))
  (set `self.canDrive` false))

(event `self.Box.OnComponentEndOverlap`
  (params (OverlappedComponent :type "PrimitiveComponent Object Reference") (OtherActor :type "Actor Object Reference") (OtherComp :type "PrimitiveComponent Object Reference") (OtherBodyIndex :type Integer))
  (`|ExecutionSequence`
    (:`then_0`
      (cast `/Game/BluePrints/Actors/BP_Civilian` OtherActor)
      (set `self.canDrive` true :!label _label))
    (:`then_1`
      (cast `/Game/BluePrints/Actors/BP_Stoplight` OtherActor)
      (goto _label))
    (:`then_2`
      (cast `/Game/BluePrints/Actors/BP_Boundary` OtherActor)
      (`self.K2_DestroyActor`))))

(fn `UserConstructionScript`)