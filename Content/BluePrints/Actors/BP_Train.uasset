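; BP_Train is a train actor that travels along a track spline and destroys what it runs into.
; On BeginPlay it finds the BP_TrainPath actor, then a Timeline alpha drives its position and rotation along the full spline length.
; Hits on its Cube zero the player BP_Car's health and trigger its death check, while other actors receive heavy generic damage.
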(event `self.ReceiveBeginPlay`
  (bind _returnvalue (`GameplayStatics.GetActorOfClass` "/Game/BluePrints/Actors/BP_TrainPath.BP_TrainPath_C"))
  (set `self.Path` _returnvalue)
  (`self.StartMoving`))

(event `StartMoving`
  (bind (_direction _alpha) (`Timeline|Timeline`)
    (:`Update`
      (bind (_returnvalue_location _returnvalue_rotation) (`KismetMathLibrary.BreakTransform` (`SplineComponent.GetTransformAtDistanceAlongSpline` (`/Game/BluePrints/Actors/BP_TrainPath.Spline` (`self.Path`)) (`KismetMathLibrary.Lerp` 0.0 (`SplineComponent.GetSplineLength` (`/Game/BluePrints/Actors/BP_TrainPath.Spline` (`self.Path`))) _alpha) "World" false)))
      (`self.K2_SetActorLocationAndRotation` _returnvalue_location _returnvalue_rotation))))

(event `self.Cube.OnComponentHit`
  (params (HitComponent :type "PrimitiveComponent Object Reference") (OtherActor :type "Actor Object Reference") (OtherComp :type "PrimitiveComponent Object Reference") (NormalImpulse :type "Vector Structure") (Hit :type "HitResult Structure (by ref)"))
  (bind _returnvalue (`GameplayStatics.GetPlayerPawn` 0))
  (if (== OtherActor _returnvalue)
    (bind _asbp_car (cast `/Game/Nathan/Player/BP_Car` _returnvalue))
    (set `/Game/Nathan/Player/BP_Car.CurrentHealth` 0.0 _asbp_car)
    (`/Game/Nathan/Player/BP_Car.CheckIfDead` _asbp_car)
    (else
      (`GameplayStatics.ApplyDamage` OtherActor 100.0 null null "/Script/Engine.DamageType"))))

(fn `UserConstructionScript`)