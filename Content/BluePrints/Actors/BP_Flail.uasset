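; BP_Flail is the car's flail weapon actor, which deals damage to actors it strikes.
; Hit events on its Child and Child2 components check that the player car's BPCFlail is the current weapon and the other actor is not BP_Car.
; A passing hit applies fixed generic damage.
; The trailing Delay follows the damage and gates nothing, so repeated hits are not throttled.
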(event `self.child2.OnComponentHit`
  (params (HitComponent :type "PrimitiveComponent Object Reference") (OtherActor :type "Actor Object Reference") (OtherComp :type "PrimitiveComponent Object Reference") (NormalImpulse :type "Vector Structure") (Hit :type "HitResult Structure (by ref)"))
  (bind _asbp_car (cast `/Game/Nathan/Player/BP_Car` (`GameplayStatics.GetPlayerPawn` 0)))
  (if (and (`/Game/BluePrints/ActorComponents/BPC_Flail.isCurrentWeapon` (`/Game/Nathan/Player/BP_Car.BPC_Flail` _asbp_car)) (!= OtherActor "/Game/Nathan/Player/BP_Car.BP_Car"))
    (`GameplayStatics.ApplyDamage` OtherActor 20.0 null null "/Script/Engine.DamageType")
    (`KismetSystemLibrary.Delay` 0.5)))

(event `self.child.OnComponentHit`
  (params (HitComponent :type "PrimitiveComponent Object Reference") (OtherActor :type "Actor Object Reference") (OtherComp :type "PrimitiveComponent Object Reference") (NormalImpulse :type "Vector Structure") (Hit :type "HitResult Structure (by ref)"))
  (bind _asbp_car (cast `/Game/Nathan/Player/BP_Car` (`GameplayStatics.GetPlayerPawn` 0)))
  (if (and (`/Game/BluePrints/ActorComponents/BPC_Flail.isCurrentWeapon` (`/Game/Nathan/Player/BP_Car.BPC_Flail` _asbp_car)) (!= OtherActor "/Game/Nathan/Player/BP_Car.BP_Car"))
    (`GameplayStatics.ApplyDamage` OtherActor 20.0 null null "/Script/Engine.DamageType")
    (`KismetSystemLibrary.Delay` 0.5)))

(fn `UserConstructionScript`)