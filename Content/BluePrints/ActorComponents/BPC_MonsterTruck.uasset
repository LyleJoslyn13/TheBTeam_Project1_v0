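; Car component for a timed monster truck power-up that temporarily enlarges the car body.
; BeginPlay caches the default relative transforms of BPCar's Cube and four wheels.
; MTPowerUp scales the Cube, pushes the unscaled wheels outward, sets IsMonsterTruck and shows a power-up message through player pawn 0.
; After a ten-second Delay it restores the cached transforms and clears both flag and message.
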(event `MTPowerUp`
  (bind _returnvalue (`GameplayStatics.GetPlayerPawn` 0))
  (bind _bp_car (`self.BP_Car`))
  (bind _fl_wheel (`/Game/Nathan/Player/BP_Car.FL_wheel` _bp_car))
  (bind _bl_wheel (`/Game/Nathan/Player/BP_Car.BL_wheel` _bp_car))
  (bind _fr_wheel (`/Game/Nathan/Player/BP_Car.FR_wheel` _bp_car))
  (bind _cube (`/Game/Nathan/Player/BP_Car.Cube` _bp_car))
  (bind _br_wheel (`/Game/Nathan/Player/BP_Car.BR_wheel` _bp_car))
  (bind _returnvalue_2 (`SceneComponent.GetRelativeTransform` _fl_wheel))
  (bind _returnvalue_3 (`SceneComponent.GetRelativeTransform` _bl_wheel))
  (bind _returnvalue_4 (`SceneComponent.GetRelativeTransform` _fr_wheel))
  (bind _returnvalue_5 (`SceneComponent.GetRelativeTransform` _br_wheel))
  (bind (_returnvalue_location _returnvalue_rotation _returnvalue_scale) (`KismetMathLibrary.BreakTransform` (`SceneComponent.GetRelativeTransform` _cube)))
  (message `/Game/BluePrints/Interfaces/BPI_PowerUp.inPowerUp` _returnvalue true)
  (set `self.isMonsterTruck` true)
  (`SceneComponent.K2_SetRelativeTransform` _cube (`KismetMathLibrary.MakeTransform` _returnvalue_location _returnvalue_rotation (* _returnvalue_scale (`self.ScaleMultiplier`))) false false)
  (`SceneComponent.K2_SetRelativeTransform` _fl_wheel (`KismetMathLibrary.MakeTransform` (`KismetMathLibrary.MakeVector` (+ (.x (.location _returnvalue_2)) (`self.ScaleChangeX`)) (- (.y (.location _returnvalue_2)) (`self.ScaleChangeY`)) (.z (.location _returnvalue_2))) (.rotation _returnvalue_2) (.scale _returnvalue_2)) false false)
  (`SceneComponent.K2_SetRelativeTransform` _bl_wheel (`KismetMathLibrary.MakeTransform` (`KismetMathLibrary.MakeVector` (- (.x (.location _returnvalue_3)) (`self.ScaleChangeX`)) (- (.y (.location _returnvalue_3)) (`self.ScaleChangeY`)) (.z (.location _returnvalue_3))) (.rotation _returnvalue_3) (.scale _returnvalue_3)) false false)
  (`SceneComponent.K2_SetRelativeTransform` _fr_wheel (`KismetMathLibrary.MakeTransform` (`KismetMathLibrary.MakeVector` (+ (.x (.location _returnvalue_4)) (`self.ScaleChangeX`)) (+ (.y (.location _returnvalue_4)) (`self.ScaleChangeY`)) (.z (.location _returnvalue_4))) (.rotation _returnvalue_4) (.scale _returnvalue_4)) false false)
  (`SceneComponent.K2_SetRelativeTransform` _br_wheel (`KismetMathLibrary.MakeTransform` (`KismetMathLibrary.MakeVector` (- (.x (.location _returnvalue_5)) (`self.ScaleChangeX`)) (+ (.y (.location _returnvalue_5)) (`self.ScaleChangeY`)) (.z (.location _returnvalue_5))) (.rotation _returnvalue_5) (.scale _returnvalue_5)) false false)
  (`KismetSystemLibrary.Delay` 10.0)
  (`SceneComponent.K2_SetRelativeTransform` (`/Game/Nathan/Player/BP_Car.Cube` _bp_car) (`self.CubeDefault`) false false)
  (`SceneComponent.K2_SetRelativeTransform` (`/Game/Nathan/Player/BP_Car.FL_wheel` _bp_car) (`self.FLDefault`) false false)
  (`SceneComponent.K2_SetRelativeTransform` (`/Game/Nathan/Player/BP_Car.BL_wheel` _bp_car) (`self.BLDefault`) false false)
  (`SceneComponent.K2_SetRelativeTransform` (`/Game/Nathan/Player/BP_Car.FR_wheel` _bp_car) (`self.FRDefault`) false false)
  (`SceneComponent.K2_SetRelativeTransform` (`/Game/Nathan/Player/BP_Car.BR_wheel` _bp_car) (`self.BRDefault`) false false)
  (message `/Game/BluePrints/Interfaces/BPI_PowerUp.inPowerUp` _returnvalue false)
  (set `self.isMonsterTruck` false))

(event `self.ReceiveBeginPlay`
  (bind _bp_car (`self.BP_Car`))
  (set `self.BLDefault` (`SceneComponent.GetRelativeTransform` (`/Game/Nathan/Player/BP_Car.BL_wheel` _bp_car)))
  (set `self.BRDefault` (`SceneComponent.GetRelativeTransform` (`/Game/Nathan/Player/BP_Car.BR_wheel` _bp_car)))
  (set `self.FLDefault` (`SceneComponent.GetRelativeTransform` (`/Game/Nathan/Player/BP_Car.FL_wheel` _bp_car)))
  (set `self.FRDefault` (`SceneComponent.GetRelativeTransform` (`/Game/Nathan/Player/BP_Car.FR_wheel` _bp_car)))
  (set `self.CubeDefault` (`SceneComponent.GetRelativeTransform` (`/Game/Nathan/Player/BP_Car.Cube` _bp_car))))