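; Player machine gun component that fires BP_FriendlyBullet actors from the character's arrow, with ammo, timed reload and looping sound control.
; Held fire runs a Delay loop whose interval shrinks until max fire rate, which unlocks random 5x crits in DealDamage.
; The timed ultimate slows global time, fires every frame without using ammo and always crits.
; EnemyKilled decrements the ult kill counter, but sets availability while kills remain, an apparently inverted check.
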(event `EnhancedInput|/Game/BluePrints/Game/Input/InputActions/IA_PrimaryAttack`
  (params (ActionValue :type Boolean) (ElapsedSeconds :type "Float (double-precision)") (TriggeredSeconds :type "Float (double-precision)") (InputAction :type "InputAction Object Reference" :default "/Game/BluePrints/Game/Input/InputActions/IA_PrimaryAttack.IA_PrimaryAttack"))
  (bind _delaytimer (`self.DelayTimer`))
  (bind _returnvalue (/ (`self.DeductValue`) 0.99))
  (bind _arrow (`/Game/Nathan/Player/BP_Car.Arrow` (`self.MainPlayerCharacter`)))
  (bind _arrow_2 (`/Game/Nathan/Player/BP_Car.Arrow` (`self.MainPlayerCharacter`)))
  (bind _returnvalue_2 (`SceneComponent.K2_GetComponentLocation` _arrow_2))
  (:`Triggered`
    (if (`self.isCurrentWeapon`)
      (set `self.isShooting` true)
      (if ActionValue
        (`|ExecutionSequence`
          (:`then_0`
            (if (not (`self.isSound`))
              (set `self.isSound` true)
              (bind _returnvalue_3 (`GameplayStatics.SpawnSoundAtLocation` "/Game/BluePrints/Sound/SC_MachineGun.SC_MachineGun" (`Actor.K2_GetActorLocation` (`self.MainPlayerCharacter`)) (struct) 1.0 1.0 0.0 null null))
              (set `self.Sound` _returnvalue_3)))
          (:`then_1`
            (if (`self.isUltActive`)
              ;[1 1 1] Ultimate Bullet Behavior
              (if (`self.isShooting`) :!label _label
                (`GameplayStatics.PlaySoundAtLocation` "/Game/BluePrints/Sound/740545__sadiquecat__wall-clock-denoised.740545__sadiquecat__wall-clock-denoised" _returnvalue_2 (struct) 1.0 1.0 0.0 null null null null)
                (`KismetSystemLibrary.Delay` 0.0) ; DONT DELETE, WITHOUT THIS NODE UNREAL WILL FREEZE
                (`|SpawnActorFromClass` "/Game/BluePrints/Actors/BP_FriendlyBullet.BP_FriendlyBullet_C" (`KismetMathLibrary.MakeTransform` _returnvalue_2 (`KismetMathLibrary.Conv_VectorToRotator` (`SceneComponent.GetForwardVector` _arrow_2))) "Undefined" "MultiplyWithRoot" null null)
                (goto _label)
                (else
                  (`AudioComponent.Stop` (`self.Sound`) :!label _label_2)
                  (set `self.isSound` false)))
              (else
                (if (>= (`self.CurrentBulletCount`) 0.0) :!label _label_3
                  (if (`self.isReloading`)
                    (goto _label_2)
                    (else
                      (`KismetSystemLibrary.Delay` _delaytimer)
                      (set `self.DeductValue` _returnvalue)
                      (bind _output_get (set `self.DelayTimer` (- _delaytimer _returnvalue)))
                      (if (<= _output_get 0.0)
                        (set `self.isROFMax` true))
                      (if (`self.isShooting`)
                        (if (> (`self.CurrentBulletCount`) 0.0)
                          (`|SpawnActorFromClass` "/Game/BluePrints/Actors/BP_FriendlyBullet.BP_FriendlyBullet_C" (`KismetMathLibrary.MakeTransform` (`SceneComponent.K2_GetComponentLocation` _arrow) (`KismetMathLibrary.Conv_VectorToRotator` (`SceneComponent.GetForwardVector` _arrow))) "Undefined" "MultiplyWithRoot" null null)
                          (set `self.CurrentBulletCount` (- (`self.CurrentBulletCount`) 1.0))
                          (goto _label_3)
                          (else
                            _)))
                      (`AudioComponent.Stop` (`self.Sound`))
                      (set `self.isSound` false)))
                  (else
                    (set `self.CurrentBulletCount` 0.0)
                    (goto _label_2))))))))))
  (:`Completed`
    ;[1 1 1] Resets Rate of fire Variables
    (if (`self.isCurrentWeapon`)
      (set `self.isShooting` false)
      (set `self.DeductValue` 0.01)
      (set `self.DelayTimer` 0.25)
      (if (not (`self.isUltActive`))
        (set `self.isROFMax` false)))))

(event `EnhancedInput|/Game/BluePrints/Game/Input/InputActions/IA_Reload`
  (params (ActionValue :type Boolean) (ElapsedSeconds :type "Float (double-precision)") (TriggeredSeconds :type "Float (double-precision)") (InputAction :type "InputAction Object Reference" :default "/Game/BluePrints/Game/Input/InputActions/IA_Reload.IA_Reload"))
  ;[1 1 1] Reload Code
  (:`Triggered`
    (if (`self.isCurrentWeapon`)
      (if ActionValue
        (if (not (>= (`self.CurrentBulletCount`) (`self.MaxBulletCount`)))
          (set `self.isReloading` true)
          (`KismetSystemLibrary.Delay` 3.0)
          (set `self.CurrentBulletCount` (`self.MaxBulletCount`))
          (set `self.isReloading` false)
          (`KismetSystemLibrary.PrintString` "FINSIHED RELOADING"))))))

(event `EnhancedInput|/Game/BluePrints/Game/Input/InputActions/IA_Ultimate`
  (params (ActionValue :type Boolean) (ElapsedSeconds :type "Float (double-precision)") (TriggeredSeconds :type "Float (double-precision)") (InputAction :type "InputAction Object Reference" :default "/Game/BluePrints/Game/Input/InputActions/IA_Ultimate.IA_Ultimate"))
  (bind _returnvalue (- (`self.CurrentUltTimer`) 1.0))
  ;[1 1 1] Ultimate variable change to make Ult Work
  (:`Triggered`
    (if (`self.isCurrentWeapon`)
      (if ActionValue
        (if (`self.isUltAvailable`)
          (`KismetSystemLibrary.PrintString` "ULTIMATE ACTIVE")
          (set `self.isUltAvailable` false)
          (set `self.isUltActive` true)
          (`GameplayStatics.SetGlobalTimeDilation` 0.75)
          (`KismetSystemLibrary.Delay` 1.0 :!label _label_4)
          (`KismetSystemLibrary.PrintString` (`KismetStringLibrary.Conv_DoubleToString` _returnvalue))
          (bind _output_get (set `self.CurrentUltTimer` _returnvalue))
          (if (<= _output_get 0.0)
            (`GameplayStatics.SetGlobalTimeDilation` 1.0)
            (set `self.isUltActive` false)
            (set `self.CurrentKillsLeftTillUlt` (`self.MaxKillsLeftTillUlt`))
            (set `self.CurrentUltTimer` (`self.MaxUltTimer`))
            (`KismetSystemLibrary.PrintString` "Ultimate Finished")
            (else
              (goto _label_4))))))))

(event `self.ReceiveBeginPlay`
  (`EnhancedInputSubsystemInterface.AddMappingContext` (pcsubsystem `EnhancedInputLocalPlayerSubsystem` (`GameplayStatics.GetPlayerController` 0)) "/Game/Nathan/Inputs/IMC_Vehicle.IMC_Vehicle" 0 (struct)))

(fn `DealDamage`
  (params (Health :type "Float (double-precision)"))
  (returns (UpdatedHealth :type "Float (double-precision)"))
  (bind _damage (`self.Damage`))
  (if (`self.isUltActive`)
    _
    (elif (`self.isROFMax`)
      (if (== (`KismetMathLibrary.RandomIntegerInRange` 0 9) 9)
        _
        (else
          (return (- Health _damage)) ; Regular Hit
        ))
      (else
        (return (- Health _damage)) ; Regular Hit
      )))
  (return (- Health (* _damage 5.0))) ; Crit Hit
)

(fn `EnemyKilled`
  ;[1 1 1] SOMEBODY PLEASE EXPLAIN WHY THIS DOESNT WORK
  (bind _output_get (set `self.CurrentKillsLeftTillUlt` (- (`self.CurrentKillsLeftTillUlt`) 1.0)))
  (`KismetSystemLibrary.PrintString` (`KismetStringLibrary.Conv_DoubleToString` _output_get))
  (if (not (<= _output_get 0.0))
    (set `self.isUltAvailable` true)))