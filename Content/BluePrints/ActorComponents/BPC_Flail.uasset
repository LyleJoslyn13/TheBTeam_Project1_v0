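; Weapon component that gives the player's car a pair of flails with a swing attack and a cooldown-gated ultimate.
; BeginPlay spawns the attached flail rig, two swing actors and two mirrored spline path actors.
; While it is the current weapon, Tick interpolates both spheres to the car's target and back for attacks.
; During the ultimate it loops both flails along the splines; otherwise they follow the rig.
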(event `self.ReceiveBeginPlay`
  (bind _returnvalue (`GameplayStatics.GetPlayerPawn` 0))
  (bind _flails (`self.Flails`))
  (bind _returnvalue_2 (`Actor.K2_GetActorLocation` _returnvalue))
  (bind (_returnvalue_x _returnvalue_y) (`KismetMathLibrary.BreakVector` (`Actor.K2_GetActorLocation` (`GameplayStatics.GetPlayerPawn` 0))))
  (bind _returnvalue_3 (`|SpawnActorFromClass` "/Game/BluePrints/Actors/BP_Flail.BP_Flail_C" (`KismetMathLibrary.MakeTransform` (`KismetMathLibrary.MakeVector` _returnvalue_x _returnvalue_y)) "Undefined" "MultiplyWithRoot" null null))
  (bind _output_get (set `self.Flails` _returnvalue_3))
  (`Actor.K2_AttachToActor` _output_get (`GameplayStatics.GetPlayerPawn` 0) "None" "SnapToTarget" "SnapToTarget" "SnapToTarget" true)
  (bind _returnvalue_4 (`|SpawnActorFromClass` "/Game/BluePrints/Actors/BP_FlailSwing.BP_FlailSwing_C" (`KismetMathLibrary.MakeTransform` (`SceneComponent.K2_GetComponentLocation` (`/Game/BluePrints/Actors/BP_Flail.child2` _flails))) "AlwaysSpawn" "MultiplyWithRoot" null null))
  (set `self.leftFlail` _returnvalue_4)
  (bind _returnvalue_5 (`|SpawnActorFromClass` "/Game/BluePrints/Actors/BP_FlailSwing.BP_FlailSwing_C" (`KismetMathLibrary.MakeTransform` (`SceneComponent.K2_GetComponentLocation` (`/Game/BluePrints/Actors/BP_Flail.child` _flails))) "AlwaysSpawn" "MultiplyWithRoot" null null))
  (set `self.rightFlail` _returnvalue_5)
  (bind _returnvalue_6 (`|SpawnActorFromClass` "/Game/BluePrints/Actors/BP_FlailPath.BP_FlailPath_C" (`KismetMathLibrary.MakeTransform` _returnvalue_2 (struct :`Yaw` -90.0)) "Undefined" "MultiplyWithRoot" null null))
  (bind _output_get_2 (set `self.LeftPath` _returnvalue_6))
  (`Actor.K2_AttachToActor` _output_get_2 _returnvalue "None" "KeepRelative" "KeepRelative" "KeepRelative" true)
  (bind _returnvalue_7 (`|SpawnActorFromClass` "/Game/BluePrints/Actors/BP_FlailPath.BP_FlailPath_C" (`KismetMathLibrary.MakeTransform` _returnvalue_2 (struct :`Yaw` 90.0)) "Undefined" "MultiplyWithRoot" null null))
  (bind _output_get_3 (set `self.RightPath` _returnvalue_7))
  (`Actor.K2_AttachToActor` _output_get_3 _returnvalue "None" "KeepRelative" "KeepRelative" "KeepRelative" true))

(event `self.ReceiveTick`
  (params (DeltaSeconds :type "Float (single-precision)"))
  (bind _flails (`self.Flails`))
  (bind _returnvalue (+ (`self.rotationSpeed`) (`GameplayStatics.GetWorldDeltaSeconds`)))
  (bind _sphere (`/Game/BluePrints/Actors/BP_FlailSwing.Sphere` (`self.rightFlail`)))
  (bind _sphere_2 (`/Game/BluePrints/Actors/BP_FlailSwing.Sphere` (`self.leftFlail`)))
  (bind _spline (`/Game/BluePrints/Actors/BP_FlailPath.Spline` (`self.RightPath`)))
  (bind _spline_2 (`/Game/BluePrints/Actors/BP_FlailPath.Spline` (`self.LeftPath`)))
  (bind _sphere_3 (`/Game/BluePrints/Actors/BP_FlailSwing.Sphere` (`self.leftFlail`)))
  (bind _sphere_4 (`/Game/BluePrints/Actors/BP_FlailSwing.Sphere` (`self.rightFlail`)))
  (bind _returnvalue_2 (`SceneComponent.K2_GetComponentLocation` (`/Game/BluePrints/Actors/BP_Flail.child` (`self.Flails`))))
  (bind _returnvalue_3 (`SceneComponent.K2_GetComponentLocation` (`/Game/BluePrints/Actors/BP_Flail.child2` (`self.Flails`))))
  (bind _returnvalue_location (`KismetMathLibrary.BreakTransform` (`SplineComponent.GetTransformAtDistanceAlongSpline` _spline (`KismetMathLibrary.Lerp` 0.0 (`SplineComponent.GetSplineLength` _spline) (`self.rotationSpeed`)) "World" false)))
  (bind _returnvalue_location_2 (`KismetMathLibrary.BreakTransform` (`SplineComponent.GetTransformAtDistanceAlongSpline` _spline_2 (`KismetMathLibrary.Lerp` 0.0 (`SplineComponent.GetSplineLength` _spline_2) (`self.rotationSpeed`)) "World" false)))
  (if (`self.isCurrentWeapon`)
    (`|ExecutionSequence`
      (:`then_0`
        (if (`self.swinging`)
          (`Actor.SetActorHiddenInGame` (`self.Flails`) true)
          (if (`self.reachedTarget`)
            ;[1 1 1] swinging
            (`|ExecutionSequence`
              (:`then_0`
                (`SceneComponent.K2_SetWorldLocation` _sphere_4 (`KismetMathLibrary.VInterpTo` (`SceneComponent.K2_GetComponentLocation` _sphere_4) _returnvalue_2 (`GameplayStatics.GetWorldDeltaSeconds`) 20.0) true true)
                (if (== (`SceneComponent.K2_GetComponentLocation` _sphere_4) _returnvalue_2 :`ErrorTolerance` 50.0)
                  (set `self.swinging` false :!label _label)
                  (set `self.reachedTarget` false)
                  (`Actor.SetActorHiddenInGame` (`self.leftFlail`) true)
                  (`Actor.SetActorHiddenInGame` (`self.rightFlail`) true)))
              (:`then_1`
                (`SceneComponent.K2_SetWorldLocation` _sphere_3 (`KismetMathLibrary.VInterpTo` (`SceneComponent.K2_GetComponentLocation` _sphere_3) _returnvalue_3 (`GameplayStatics.GetWorldDeltaSeconds`) 20.0) true true)
                (if (== (`SceneComponent.K2_GetComponentLocation` _sphere_3) _returnvalue_3 :`ErrorTolerance` 50.0)
                  (goto _label))))
            (else
              (`|ExecutionSequence`
                (:`then_0`
                  (`Actor.SetActorHiddenInGame` (`self.leftFlail`) false)
                  (`SceneComponent.K2_SetWorldLocation` _sphere_2 (`KismetMathLibrary.VInterpTo` (`SceneComponent.K2_GetComponentLocation` _sphere_2) (`self.targetLocation`) (`GameplayStatics.GetWorldDeltaSeconds`) 10.0) true true)
                  (if (== (`SceneComponent.K2_GetComponentLocation` _sphere_2) (`self.targetLocation`) :`ErrorTolerance` 50.0)
                    (set `self.reachedTarget` true :!label _label_2)))
                (:`then_1`
                  (`Actor.SetActorHiddenInGame` (`self.rightFlail`) false)
                  (`SceneComponent.K2_SetWorldLocation` _sphere (`KismetMathLibrary.VInterpTo` (`SceneComponent.K2_GetComponentLocation` _sphere) (`self.targetLocation`) (`GameplayStatics.GetWorldDeltaSeconds`) 10.0) true true)
                  (if (== (`SceneComponent.K2_GetComponentLocation` _sphere) (`self.targetLocation`) :`ErrorTolerance` 50.0)
                    (goto _label_2))))))
          (elif (`self.ulting`)
            ;[1 1 1] utlimate
            (`Actor.SetActorHiddenInGame` (`self.Flails`) true)
            (if (>= _returnvalue 1.0)
              (set `self.rotationSpeed` 0.0)
              (else
                (set `self.rotationSpeed` _returnvalue)))
            (`Actor.K2_SetActorLocation` (`self.leftFlail`) _returnvalue_location_2 true true)
            (`Actor.K2_SetActorLocation` (`self.rightFlail`) _returnvalue_location true true)
            (set `self.UltTimer` (+ (`self.UltTimer`) (`GameplayStatics.GetWorldDeltaSeconds`)))
            (if (>= (`self.UltTimer`) 8.0)
              (set `self.UltCD` 60.0)
              (`Actor.SetActorHiddenInGame` (`self.Flails`) false)
              (set `self.ulting` false))
            (else
              ;[1 1 1] default flail movement
              (`Actor.SetActorHiddenInGame` (`self.Flails`) false)
              (`Actor.K2_SetActorLocation` (`self.leftFlail`) (`SceneComponent.K2_GetComponentLocation` (`/Game/BluePrints/Actors/BP_Flail.child2` _flails)) true true)
              (`Actor.K2_SetActorLocation` (`self.rightFlail`) (`SceneComponent.K2_GetComponentLocation` (`/Game/BluePrints/Actors/BP_Flail.child` _flails)) true true)))))
      (:`then_1`
        (if (not (<= (`self.UltCD`) 0.0))
          (set `self.UltCD` (- (`self.UltCD`) (`GameplayStatics.GetWorldDeltaSeconds`))))))
    (else
      (`Actor.SetActorHiddenInGame` (`self.Flails`) true)
      (`Actor.SetActorHiddenInGame` (`self.leftFlail`) true)
      (`Actor.SetActorHiddenInGame` (`self.rightFlail`) true))))

(event `EnhancedInput|/Game/BluePrints/Game/Input/InputActions/IA_Ultimate`
  (params (ActionValue :type Boolean) (ElapsedSeconds :type "Float (double-precision)") (TriggeredSeconds :type "Float (double-precision)") (InputAction :type "InputAction Object Reference" :default "/Game/BluePrints/Game/Input/InputActions/IA_Ultimate.IA_Ultimate"))
  (:`Started`
    (if (`self.isCurrentWeapon`)
      (if (<= (`self.UltCD`) 0.0)
        (set `self.ulting` true)
        (`Actor.SetActorHiddenInGame` (`self.leftFlail`) false)
        (`Actor.SetActorHiddenInGame` (`self.rightFlail`) false)
        (`KismetSystemLibrary.Delay` 8.0)
        (`Actor.SetActorHiddenInGame` (`self.leftFlail`) true)
        (`Actor.SetActorHiddenInGame` (`self.rightFlail`) true)))))

(event `EnhancedInput|/Game/BluePrints/Game/Input/InputActions/IA_PrimaryAttack`
  (params (ActionValue :type Boolean) (ElapsedSeconds :type "Float (double-precision)") (TriggeredSeconds :type "Float (double-precision)") (InputAction :type "InputAction Object Reference" :default "/Game/BluePrints/Game/Input/InputActions/IA_PrimaryAttack.IA_PrimaryAttack"))
  (:`Started`
    (if (`self.isCurrentWeapon`)
      (if (not (`self.swinging`))
        (bind _asbp_car (cast `/Game/Nathan/Player/BP_Car` (`GameplayStatics.GetPlayerPawn` 0)))
        (set `self.targetLocation` (`/Game/Nathan/Player/BP_Car.TargetLocation` _asbp_car))
        (set `self.swinging` true)))))