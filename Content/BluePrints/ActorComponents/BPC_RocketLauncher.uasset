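; Actor component that gives the player character a rocket launcher and a meteor ultimate.
; Primary attack traces from the mouse cursor, spawns BP_BasicRocket at the launch arrow and sets its velocity along the vector from hit point to character.
; Ultimate input spawns BP_Meteor when available.
; Tick-driven Delays restore firing and manage ultimate flags; the homing branch is empty, and CanUlt is never cleared here.
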(event `self.ReceiveTick`
  (params (DeltaSeconds :type "Float (single-precision)"))
  (`|ExecutionSequence`
    (:`then_0`
      (if (not (`self.canShoot`))
        (`KismetSystemLibrary.Delay` 2.0)
        (set `self.canShoot` true)))
    (:`then_1`
      (if (`self.canShootHoming`)
        _))
    (:`then_2`
      (if (not (and (`self.canUlt`) (`self.isUlting`)))
        (`KismetSystemLibrary.Delay` 5.0)
        (`KismetSystemLibrary.PrintString` "ULT READY")
        (set `self.canUlt` true)))
    (:`then_3`
      (if (`self.isUlting`)
        (`KismetSystemLibrary.Delay` 10.0)
        (set `self.isUlting` false)))))

(event `EnhancedInput|/Game/BluePrints/Game/Input/InputActions/IA_PrimaryAttack`
  (params (ActionValue :type Boolean) (ElapsedSeconds :type "Float (double-precision)") (TriggeredSeconds :type "Float (double-precision)") (InputAction :type "InputAction Object Reference" :default "/Game/BluePrints/Game/Input/InputActions/IA_PrimaryAttack.IA_PrimaryAttack"))
  (bind (_worldlocation _worlddirection) (`PlayerController.DeprojectMousePositionToWorld` (`GameplayStatics.GetPlayerController` 0)))
  (bind _launcharrow (`/Game/BluePrints/Players/BP_MainPlayerCharacter.LaunchArrow` (`self.MainPlayerCharacter`)))
  (:`Triggered`
    (if (`self.canShoot`)
      (set `self.canShoot` false)
      (bind _outhit (`KismetSystemLibrary.LineTraceSingle` _worldlocation (+ _worldlocation (* _worlddirection 10000.0)) "TraceTypeQuery1"))
      (bind (_bblockinghit _binitialoverlap _time _distance _location _impactpoint _normal _impactnormal _physmat _hitactor _hitcomponent) (`GameplayStatics.BreakHitResult` _outhit))
      (set `self.Hit Component` _hitcomponent)
      (bind _returnvalue (`|SpawnActorFromClass` "/Game/BluePrints/Actors/BP_BasicRocket.BP_BasicRocket_C" (`KismetMathLibrary.MakeTransform` (`SceneComponent.K2_GetComponentLocation` _launcharrow) (`KismetMathLibrary.Conv_VectorToRotator` (`SceneComponent.GetForwardVector` _launcharrow))) "Undefined" "MultiplyWithRoot" null null))
      (set `MovementComponent.Velocity` (* (`KismetMathLibrary.Normal` (- (`Actor.K2_GetActorLocation` (`self.MainPlayerCharacter`)) _location)) 1000.0) (`/Game/BluePrints/Actors/BP_BasicRocket.ProjectileMovement` _returnvalue)))))

(event `EnhancedInput|/Game/BluePrints/Game/Input/InputActions/IA_Ultimate`
  (params (ActionValue :type Boolean) (ElapsedSeconds :type "Float (double-precision)") (TriggeredSeconds :type "Float (double-precision)") (InputAction :type "InputAction Object Reference" :default "/Game/BluePrints/Game/Input/InputActions/IA_Ultimate.IA_Ultimate"))
  (:`Triggered`
    (if ActionValue
      (if (`self.canUlt`)
        (set `self.isUlting` true)
        (`|SpawnActorFromClass` "/Game/BluePrints/Actors/BP_Meteor.BP_Meteor_C" (`KismetMathLibrary.MakeTransform` (0.0 0.0 0.0)) "Undefined" "MultiplyWithRoot" null null)))))