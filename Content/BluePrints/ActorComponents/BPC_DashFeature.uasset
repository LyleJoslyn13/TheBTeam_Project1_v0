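; Actor component that gives its owning character a dash, triggered by the IA_Dash Enhanced Input action.
; The dash targets a point a fixed distance along the character's velocity direction, so standing still gives no displacement.
; A DelayUntilNextTick loop replaces Tick, lerping location with swept moves as DashAlpha advances by DashSpeed and delta time.
; CanDash blocks re-triggering until the alpha completes, with no further cooldown.
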(event `EnhancedInput|/Game/BluePrints/Game/Input/InputActions/IA_Dash`
  (params (ActionValue :type Boolean) (ElapsedSeconds :type "Float (double-precision)") (TriggeredSeconds :type "Float (double-precision)") (InputAction :type "InputAction Object Reference" :default "/Game/BluePrints/Game/Input/InputActions/IA_Dash.IA_Dash"))
  (bind _owningcharacter (`self.owningCharacter`))
  ;[1 1 1] Good Dash
  (:`Triggered`
    (if ActionValue
      (if (`self.CanDash`)
        (set `self.CanDash` false)
        (bind _output_get (set `self.TempLocation` (`Actor.K2_GetActorLocation` _owningcharacter)))
        (set `self.DashToLocation` (+ (* (`KismetMathLibrary.Normal` (`Actor.GetVelocity` _owningcharacter)) 1000.0) _output_get))
        (set `self.IsDashing` true)
        (if (`self.IsDashing`) :!label _label
          (`Actor.K2_SetActorLocation` (`self.owningCharacter`) (`KismetMathLibrary.VLerp` (`self.TempLocation`) (`self.DashToLocation`) (`self.DashAlpha`)) true false)
          (bind _output_get_2 (set `self.DashAlpha` (+ (`self.DashAlpha`) (* (`self.DashSpeed`) (`GameplayStatics.GetWorldDeltaSeconds`)))))
          (if (>= _output_get_2 1.0)
            (set `self.CanDash` true)
            (set `self.IsDashing` false)
            (set `self.DashAlpha` 0.0))
          (`KismetSystemLibrary.DelayUntilNextTick`)
          (goto _label))))))