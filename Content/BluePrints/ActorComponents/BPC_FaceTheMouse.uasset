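; Actor component that turns the owning character's Arrow component to face the mouse cursor.
; Each tick it traces under player 0's cursor on TraceTypeQuery3 and, on a blocking hit, takes the direction to the hit point.
; That direction starts from the arrow's relative location with Z zeroed, rather than its world location.
; The arrow's relative yaw interpolates smoothly toward the resulting yaw.
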(event `self.ReceiveTick`
  (params (DeltaSeconds :type "Float (single-precision)"))
  (bind _arrow (`/Game/Nathan/Player/BP_Car.Arrow` (`self.OwningCharacterReference`)))
  (bind (_returnvalue_roll _returnvalue_pitch _returnvalue_yaw) (`KismetMathLibrary.BreakRotator` (`KismetMathLibrary.Conv_VectorToRotator` (`KismetMathLibrary.GetDirectionUnitVector` (`self.ArrowLocation`) (`self.MouseLocation`)))))
  (bind (_bblockinghit _binitialoverlap _time _distance _location) (`GameplayStatics.BreakHitResult` (`PlayerController.GetHitResultUnderCursorByChannel` (`GameplayStatics.GetPlayerController` 0) "TraceTypeQuery3" true)))
  (bind (_relativelocation_x _relativelocation_y) (`KismetMathLibrary.BreakVector` (`SceneComponent.RelativeLocation` _arrow)))
  (bind (_relativerotation_roll _relativerotation_pitch _relativerotation_yaw) (`KismetMathLibrary.BreakRotator` (`SceneComponent.RelativeRotation` _arrow)))
  (if _bblockinghit
    (set `self.ArrowLocation` (`KismetMathLibrary.MakeVector` _relativelocation_x _relativelocation_y))
    (set `self.MouseLocation` _location)
    (`SceneComponent.K2_SetRelativeRotation` _arrow (`KismetMathLibrary.RInterpTo` (`KismetMathLibrary.MakeRotator` 0.0 0.0 _relativerotation_yaw) (`KismetMathLibrary.MakeRotator` 0.0 0.0 _returnvalue_yaw) (`GameplayStatics.GetWorldDeltaSeconds`) 10.0) false false)))