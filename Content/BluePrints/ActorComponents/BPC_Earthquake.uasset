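; BPC_Earthquake is a short-lived actor component that pulses area damage to BP_PoliceEnemy actors, then destroys itself a few seconds after BeginPlay.
; Tick calls Pulse through a CanPulse flag and Delay, so it repeats at half-second intervals.
; Pulse loops over all police enemies and damages each one passing an owner-distance check against PulseRange, although GetDistanceTo shows no target actor.
; The Earthquake event is an empty stub.
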(event `self.ReceiveBeginPlay`
  (`KismetSystemLibrary.Delay` 5.0)
  (`self.K2_DestroyComponent`))

(event `self.ReceiveTick`
  (params (DeltaSeconds :type "Float (single-precision)"))
  (if (`self.canPulse`)
    (set `self.canPulse` false)
    (`self.Pulse`)
    (`KismetSystemLibrary.Delay` 0.5)
    (set `self.canPulse` true)))

(event `Earthquake`)

(fn `Pulse`
  (bind _outactors (`GameplayStatics.GetAllActorsOfClass` "/Game/BluePrints/Enemys/BP_PoliceEnemy.BP_PoliceEnemy_C"))
  (for _array_element _outactors
    (if (<= (`Actor.GetDistanceTo` (`self.GetOwner`) null) (`self.pulseRange`))
      (`GameplayStatics.ApplyDamage` _array_element 10.0))))