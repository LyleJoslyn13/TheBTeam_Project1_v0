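; BP_Flail is a flail weapon Blueprint with a master and child component joined by a physics constraint.
; When swung during an attack, it breaks the constraint and launches the child along its own forward vector with an impulse.
; After a short delay it re-binds the child to the master through the constraint.
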(event `swing`
  (bind _child (`self.child`))
  (bind _physicsconstraint (`self.PhysicsConstraint`))
  (if (`self.attack`)
    (`PhysicsConstraintComponent.BreakConstraint` _physicsconstraint)
    (`PrimitiveComponent.AddImpulse` _child (`KismetMathLibrary.GetForwardVector` (`SceneComponent.K2_GetComponentRotation` _child)) "None" false)
    (`KismetSystemLibrary.Delay` 0.5)
    (`PhysicsConstraintComponent.SetConstrainedComponents` _physicsconstraint (`self.master`) "None" (`self.child`) "None")))

(fn `UserConstructionScript`)