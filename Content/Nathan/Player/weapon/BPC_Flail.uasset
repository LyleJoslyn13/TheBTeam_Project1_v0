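; Player weapon component that gives the player pawn a pair of swinging flails.
; BeginPlay attaches a BP_Flail rig to the pawn and spawns left and right BP_FlailSwing actors at its child points, which they follow while idle.
; IA_Swing snapshots BP_Car's TargetLocation.
; Tick then shows both flails and interpolates their spheres to it with sweeps, returning them faster and hiding both once either gets back.
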(event `self.ReceiveBeginPlay`
  (bind _flails (`self.Flails`))
  (bind (_returnvalue_x _returnvalue_y _returnvalue_z) (`KismetMathLibrary.BreakVector` (`Actor.K2_GetActorLocation` (`GameplayStatics.GetPlayerPawn` 0))))
  (bind _returnvalue (`|SpawnActorFromClass` "/Game/Nathan/Player/weapon/BP_Flail.BP_Flail_C" (`KismetMathLibrary.MakeTransform` (`KismetMathLibrary.MakeVector` _returnvalue_x _returnvalue_y (- _returnvalue_z 100.0))) "Undefined" "MultiplyWithRoot" null null))
  (bind _output_get (set `self.Flails` _returnvalue))
  (`Actor.K2_AttachToActor` _output_get (`GameplayStatics.GetPlayerPawn` 0) "None" "KeepRelative" "KeepRelative" "KeepRelative" true)
  (bind _returnvalue_2 (`|SpawnActorFromClass` "/Game/Nathan/Player/weapon/BP_FlailSwing.BP_FlailSwing_C" (`KismetMathLibrary.MakeTransform` (`SceneComponent.K2_GetComponentLocation` (`/Game/Nathan/Player/weapon/BP_Flail.child2` _flails))) "AlwaysSpawn" "MultiplyWithRoot" null null))
  (set `self.leftFlail` _returnvalue_2)
  (bind _returnvalue_3 (`|SpawnActorFromClass` "/Game/Nathan/Player/weapon/BP_FlailSwing.BP_FlailSwing_C" (`KismetMathLibrary.MakeTransform` (`SceneComponent.K2_GetComponentLocation` (`/Game/Nathan/Player/weapon/BP_Flail.child` _flails))) "AlwaysSpawn" "MultiplyWithRoot" null null))
  (set `self.rightFlail` _returnvalue_3))

(event `self.ReceiveTick`
  (params (DeltaSeconds :type "Float (single-precision)"))
  (bind _returnvalue (`GameplayStatics.GetWorldDeltaSeconds`))
  (bind _returnvalue_2 (`GameplayStatics.GetWorldDeltaSeconds`))
  (bind _flails (`self.Flails`))
  (bind _sphere (`/Game/Nathan/Player/weapon/BP_FlailSwing.Sphere` (`self.rightFlail`)))
  (bind _sphere_2 (`/Game/Nathan/Player/weapon/BP_FlailSwing.Sphere` (`self.leftFlail`)))
  (bind _sphere_3 (`/Game/Nathan/Player/weapon/BP_FlailSwing.Sphere` (`self.leftFlail`)))
  (bind _sphere_4 (`/Game/Nathan/Player/weapon/BP_FlailSwing.Sphere` (`self.rightFlail`)))
  (bind _returnvalue_3 (`SceneComponent.K2_GetComponentLocation` (`/Game/Nathan/Player/weapon/BP_Flail.child` (`self.Flails`))))
  (bind _returnvalue_4 (`SceneComponent.K2_GetComponentLocation` (`/Game/Nathan/Player/weapon/BP_Flail.child2` (`self.Flails`))))
  (if (`self.swinging`)
    (if (`self.reachedTarget`)
      (`|ExecutionSequence`
        (:`then_0`
          (`SceneComponent.K2_SetWorldLocation` _sphere_4 (`KismetMathLibrary.VInterpTo` (`SceneComponent.K2_GetComponentLocation` _sphere_4) _returnvalue_3 _returnvalue 20.0) true true)
          (if (== (`SceneComponent.K2_GetComponentLocation` _sphere_4) _returnvalue_3 :`ErrorTolerance` 50.0)
            (set `self.swinging` false :!label _label)
            (set `self.reachedTarget` false)
            (`Actor.SetActorHiddenInGame` (`self.leftFlail`) true)
            (`Actor.SetActorHiddenInGame` (`self.rightFlail`) true)))
        (:`then_1`
          (`SceneComponent.K2_SetWorldLocation` _sphere_3 (`KismetMathLibrary.VInterpTo` (`SceneComponent.K2_GetComponentLocation` _sphere_3) _returnvalue_4 _returnvalue 20.0) true true)
          (if (== (`SceneComponent.K2_GetComponentLocation` _sphere_3) _returnvalue_4 :`ErrorTolerance` 50.0)
            (goto _label))))
      (else
        (`|ExecutionSequence`
          (:`then_0`
            (`Actor.SetActorHiddenInGame` (`self.leftFlail`) false)
            (`SceneComponent.K2_SetWorldLocation` _sphere_2 (`KismetMathLibrary.VInterpTo` (`SceneComponent.K2_GetComponentLocation` _sphere_2) (`self.targetLocation`) _returnvalue_2 10.0) true true)
            (if (== (`SceneComponent.K2_GetComponentLocation` _sphere_2) (`self.targetLocation`) :`ErrorTolerance` 50.0)
              (set `self.reachedTarget` true)))
          (:`then_1`
            (`Actor.SetActorHiddenInGame` (`self.rightFlail`) false)
            (`SceneComponent.K2_SetWorldLocation` _sphere (`KismetMathLibrary.VInterpTo` (`SceneComponent.K2_GetComponentLocation` _sphere) (`self.targetLocation`) _returnvalue_2 10.0) true true)
            (if (== (`SceneComponent.K2_GetComponentLocation` _sphere) (`self.targetLocation`) :`ErrorTolerance` 50.0)
              (set `self.reachedTarget` true))))))
    (else
      (`Actor.K2_SetActorLocation` (`self.leftFlail`) (`SceneComponent.K2_GetComponentLocation` (`/Game/Nathan/Player/weapon/BP_Flail.child2` _flails)) true true)
      (`Actor.K2_SetActorLocation` (`self.rightFlail`) (`SceneComponent.K2_GetComponentLocation` (`/Game/Nathan/Player/weapon/BP_Flail.child` _flails)) true true))))

(event `EnhancedInput|/Game/Nathan/Inputs/IA_Swing`
  (params (ActionValue :type Boolean) (ElapsedSeconds :type "Float (double-precision)") (TriggeredSeconds :type "Float (double-precision)") (InputAction :type "InputAction Object Reference" :default "/Game/Nathan/Inputs/IA_Swing.IA_Swing"))
  (:`Started`
    (if (not (`self.swinging`))
      (bind _asbp_car (cast `/Game/Nathan/Player/BP_Car` (`GameplayStatics.GetPlayerPawn` 0)))
      (set `self.targetLocation` (`/Game/Nathan/Player/BP_Car.TargetLocation` _asbp_car))
      (set `self.swinging` true))))