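; BP_Car is a player-driven, physics-based car that adds face-the-mouse and machine gun components on BeginPlay.
; Each tick, four wheel line traces apply spring-like suspension and, when grounded, forward drive forces to the Box body.
; Enhanced Input eases a decaying throttle value and steers through torque under a throttle-scaled angular velocity cap.
; Braking triggers burnout boosts, drifting with a higher turn cap, or slowdown, while yaw spin decays without steering.
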(event `EnhancedInput|/Game/Nathan/Inputs/IA_Brake`
  (params (ActionValue :type Boolean) (ElapsedSeconds :type "Float (double-precision)") (TriggeredSeconds :type "Float (double-precision)") (InputAction :type "InputAction Object Reference" :default "/Game/Nathan/Inputs/IA_Brake.IA_Brake"))
  (:`Triggered`
    (if (and (> (`|GetInputActionValue`) 0.0) (< (`KismetMathLibrary.Abs` (`self.Acceleration`)) 0.05))
      (set `self.Burnout` true)
      (elif (> (`self.Acceleration`) 20.0)
        (set `self.Drifting` true)
        (else
          (set `self.AccelerationInput` (`KismetMathLibrary.FInterpTo` (`self.AccelerationInput`) 0.0 (`GameplayStatics.GetWorldDeltaSeconds`) 0.98))))))
  (:`Completed`
    (if (`self.Burnout`)
      (set `self.AccelerationInput` 1.8)
      (set `self.Burnout` false))))

(event `EnhancedInput|/Game/Nathan/Inputs/IA_Steer`
  (params (ActionValue :type "Float (double-precision)") (ElapsedSeconds :type "Float (double-precision)") (TriggeredSeconds :type "Float (double-precision)") (InputAction :type "InputAction Object Reference" :default "/Game/Nathan/Inputs/IA_Steer.IA_Steer"))
  (bind _box (`self.Box`))
  (:`Triggered`
    (if (> (`KismetMathLibrary.Abs` (`self.AccelerationInput`)) 0.05)
      (if (`self.Drifting`)
        (`PrimitiveComponent.SetPhysicsMaxAngularVelocityInRadians` _box (* 1.6 (`self.AccelerationInput`) 2.0) false "None")
        (else
          (`PrimitiveComponent.SetPhysicsMaxAngularVelocityInRadians` _box (* 0.8 (`self.AccelerationInput`) 2.0) false "None")))
      (`PrimitiveComponent.AddTorqueInRadians` _box (`KismetMathLibrary.MakeVector` 0.0 0.0 (* ActionValue 500000.0)) "None" false)
      (else
        (`PrimitiveComponent.SetPhysicsAngularVelocityInRadians` _box (0.0 0.0 0.0) false "None")))))

(event `self.ReceiveBeginPlay`
  (bind _returnvalue (`GameplayStatics.GetPlayerController` 0))
  (`EnhancedInputSubsystemInterface.AddMappingContext` (pcsubsystem `EnhancedInputLocalPlayerSubsystem` _returnvalue) "/Game/Nathan/Inputs/IMC_Vehicle.IMC_Vehicle" 0 (struct))
  (set `PlayerController.bShowMouseCursor` true _returnvalue)
  (`AddComponent|NODE_AddBPC_FaceTheMouse-0` :`OwningCharacterReference` self)
  (`AddComponent|NODE_AddBPC_MachineGun-0` :`MainPlayerCharacter` self))

(event `EnhancedInput|/Game/Nathan/Inputs/IA_Accelerate`
  (params (ActionValue :type "Float (double-precision)") (ElapsedSeconds :type "Float (double-precision)") (TriggeredSeconds :type "Float (double-precision)") (InputAction :type "InputAction Object Reference" :default "/Game/Nathan/Inputs/IA_Accelerate.IA_Accelerate"))
  (:`Triggered`
    (if (not (`|GetInputActionValue`))
      (set `self.AccelerationInput` (`KismetMathLibrary.FInterpTo` (`self.AccelerationInput`) ActionValue (`GameplayStatics.GetWorldDeltaSeconds`) 0.5)))))

(event `self.ReceiveTick`
  (params (DeltaSeconds :type "Float (single-precision)"))
  (bind _box (`self.Box`))
  (bind (_returnvalue_x _returnvalue_y _returnvalue_z) (`KismetMathLibrary.BreakVector` (`PrimitiveComponent.GetPhysicsAngularVelocityInRadians` (`self.Box`) "None")))
  (bind _returnvalue (- (`self.AngularVelocity`) (`GameplayStatics.GetWorldDeltaSeconds`)))
  (bind _returnvalue_2 (+ (`GameplayStatics.GetWorldDeltaSeconds`) (`self.AngularVelocity`)))
  (`self.SuspensionCast` (`self.FL_wheel`))
  (`self.SuspensionCast` (`self.BR_wheel`))
  (`self.SuspensionCast` (`self.BL_wheel`))
  (`self.SuspensionCast` (`self.FR_wheel`))
  (`self.CalcAccel`)
  (set `self.AngularVelocity` _returnvalue_z)
  (`|ExecutionSequence`
    (:`then_0`
      (if (< (`KismetMathLibrary.Abs` (`self.AngularVelocity`)) 0.05)
        (set `self.Drifting` false)
        (set `self.AngularVelocity` 0.0)))
    (:`then_1`
      (if (and (!= (`self.AngularVelocity`) 0.0) (== 0.0 (`|GetInputActionValue`)))
        (if (> (`self.AngularVelocity`) 0.0)
          (`PrimitiveComponent.SetAllPhysicsAngularVelocityInRadians` (`self.Box`) (`KismetMathLibrary.MakeVector` 0.0 0.0 _returnvalue) false)
          (`PrimitiveComponent.SetPhysicsMaxAngularVelocityInRadians` _box _returnvalue false "None")
          (else
            (`PrimitiveComponent.SetAllPhysicsAngularVelocityInRadians` (`self.Box`) (`KismetMathLibrary.MakeVector` 0.0 0.0 _returnvalue_2) false)
            (`PrimitiveComponent.SetPhysicsMaxAngularVelocityInRadians` _box _returnvalue_2 false "None")))))))

(fn `CalcAccel`
  (bind _accelerationinput (`self.AccelerationInput`))
  (set `self.Acceleration` (* (`KismetMathLibrary.Lerp` 0.0 100.0 _accelerationinput) _accelerationinput))
  (set `self.AccelerationInput` (`KismetMathLibrary.FInterpTo` (`self.AccelerationInput`) 0.0 (`GameplayStatics.GetWorldDeltaSeconds`) 0.3)))

(fn `SuspensionCast`
  (params (WheelComp :type "SceneComponent Object Reference"))
  (bind _returnvalue (`SceneComponent.K2_GetComponentLocation` WheelComp))
  (bind _box (`self.Box`))
  (bind _outhit (`KismetSystemLibrary.LineTraceSingle` :`Start` _returnvalue :`End` (+ _returnvalue (* (`SceneComponent.GetUpVector` WheelComp) -60.0)) :`TraceChannel` "TraceTypeQuery1" :`DrawDebugType` "ForOneFrame"))
  (bind (_bblockinghit _binitialoverlap _time _distance _location _impactpoint _normal _impactnormal _physmat _hitactor _hitcomponent _hitbonename _bonename _hititem _elementindex _faceindex _tracestart _traceend) (`GameplayStatics.BreakHitResult` _outhit))
  (if _bblockinghit
    (`PrimitiveComponent.AddForceAtLocation` (`self.Box`) (* (- 1.0 (`KismetMathLibrary.NormalizeToRange` _distance 0.0 60.0)) (`KismetMathLibrary.GetDirectionUnitVector` _traceend _tracestart) 100000.0) (`SceneComponent.K2_GetComponentLocation` (`local.WheelComp`)) "None")
    (`PrimitiveComponent.AddForceAtLocation` (`self.Box`) (* (`SceneComponent.GetForwardVector` _box) 2000.0 (`PrimitiveComponent.GetMass` _box) (`self.AccelerationInput`)) (`SceneComponent.K2_GetComponentLocation` (`local.WheelComp`)) "None")))

(fn `UserConstructionScript`)