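; BP_Tank is an enemy tank that hunts and fires at the player's BP_Car when its PawnSensing component sees it.
; Each sighting turns the actor's yaw and the Body's pitch and yaw toward the car using RInterpTo, then issues AIMoveTo with a stand-off acceptance radius.
; In parallel, a Delay paces shooting, spawning a BP_Bullet at BulletSpawn a few seconds after a sighting.
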(event `self.PawnSensing.OnSeePawn`
  (params (Pawn :type "Pawn Object Reference"))
  (bind _asbp_car (cast `/Game/Nathan/Player/BP_Car` Pawn))
  (`|ExecutionSequence`
    (:`then_0`
      (bind (_returnvalue_roll _returnvalue_pitch _returnvalue_yaw) (`KismetMathLibrary.BreakRotator` (`KismetMathLibrary.RInterpTo` (`self.K2_GetActorRotation`) (`KismetMathLibrary.FindLookAtRotation` (`self.K2_GetActorLocation`) (`self.K2_GetActorLocation` _asbp_car)) (`GameplayStatics.GetWorldDeltaSeconds`) 100.0)))
      (`SceneComponent.K2_SetWorldRotation` (`self.body`) (`KismetMathLibrary.MakeRotator` 0.0 _returnvalue_pitch _returnvalue_yaw) false false)
      (`self.K2_SetActorRotation` (`KismetMathLibrary.MakeRotator` 0.0 0.0 _returnvalue_yaw))
      (`|AIMoveTo` self (0.0 0.0 0.0) _asbp_car 1000.0))
    (:`then_1`
      (`KismetSystemLibrary.Delay` 3.0)
      (`|SpawnActorFromClass` "/Game/Nathan/Enemies/BP_Bullet.BP_Bullet_C" (`SceneComponent.K2_GetComponentToWorld` (`self.bulletSpawn`)) "AlwaysSpawn" "MultiplyWithRoot" null null))))

(fn `UserConstructionScript`)